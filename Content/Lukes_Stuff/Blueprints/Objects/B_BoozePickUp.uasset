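; B_BoozePickUp is a booze pickup that disappears when the player's pawn touches it and reappears after a delay.
; On overlap with player pawn 0, it turns off overlap events on BoxOverlap and hides Mesh, then restores both after a fixed 12-second Delay.
; The actor is never destroyed, and this Blueprint applies no effect to the player itself.
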(event `self.ReceiveActorBeginOverlap`
  (params (OtherActor :type "Actor Object Reference"))
  (bind _boxoverlap (`self.BoxOverlap`))
  (bind _mesh (`self.Mesh`))
  (if (== OtherActor (`GameplayStatics.GetPlayerPawn` 0))
    (set `PrimitiveComponent.bGenerateOverlapEvents` false _boxoverlap)
    (`SceneComponent.SetVisibility` _mesh false false)
    (`KismetSystemLibrary.Delay` 12.0)
    (set `PrimitiveComponent.bGenerateOverlapEvents` true _boxoverlap)
    (`SceneComponent.SetVisibility` _mesh true false)))

(fn `UserConstructionScript`)